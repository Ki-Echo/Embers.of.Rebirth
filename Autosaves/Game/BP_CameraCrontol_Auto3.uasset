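; BP_CameraCrontol is an actor that sets up the game camera and its input for the first player when play begins.
; BeginPlay adds the IMC_Camera mapping context through Enhanced Input, then spawns a BP_Camera at the actor's own location and makes it the view target.
; Overlap, tick and construction logic are empty, so it only handles this one-time setup.
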(event `self.ReceiveBeginPlay`
  (`|ExecutionSequence`
    (:`then_0`
      (bind _asplayer_controller (cast `PlayerController` (`GameplayStatics.GetPlayerController` 0)))
      (bind _returnvalue (pcsubsystem `EnhancedInputLocalPlayerSubsystem` _asplayer_controller))
      (`/Engine/EditorBlueprintResources/StandardMacros.IsValid` _returnvalue
        (:`Is Valid`
          (`EnhancedInputSubsystemInterface.AddMappingContext` _returnvalue "/Game/IMC_Camera.IMC_Camera" 0 (struct)))))
    (:`then_1`
      (bind _returnvalue_2 (`|SpawnActorFromClass` "/Game/BP_Camera.BP_Camera_C" (`KismetMathLibrary.MakeTransform` (`self.K2_GetActorLocation` self)) "Undefined" "MultiplyWithRoot" self null))
      (`PlayerController.SetViewTargetWithBlend` (`GameplayStatics.GetPlayerController` 0) _returnvalue_2 0.0 "VTBlend_Linear" 0.0 false))))

(event `EnhancedInput|/Game/IA_LeftAndRight`
  (params (ActionValue :type Boolean) (ElapsedSeconds :type "Float (double-precision)") (TriggeredSeconds :type "Float (double-precision)") (InputAction :type "InputAction Object Reference" :default "/Game/IA_LeftAndRight.IA_LeftAndRight")))

(fn `UserConstructionScript`)