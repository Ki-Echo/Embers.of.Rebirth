(event `self.ReceiveBeginPlay`
  (bind _asrtscamera (cast `/Game/RTSCamera/RTSCamera` (`Actor.GetOwner`)))
  (set `self.As RTSCamera` _asrtscamera)
  (set `self.Camera` (`/Game/RTSCamera/RTSCamera.Camera` _asrtscamera)))

(event `Preview Loop`
  (bind (_returnvalue_location _returnvalue_rotation) (`KismetMathLibrary.BreakTransform` (`SceneComponent.K2_GetComponentToWorld` (`self.Camera`))))
  (bind _outhit (`KismetSystemLibrary.LineTraceSingle` :`Start` _returnvalue_location :`End` (+ _returnvalue_location (* (`KismetMathLibrary.GetForwardVector` _returnvalue_rotation) 700.0)) :`TraceChannel` "TraceTypeQuery1" :`DrawDebugType` "ForDuration"))
  (if true
    (`|ExecutionSequence`
      (:`then_0`
        (`/Engine/EditorBlueprintResources/StandardMacros.DoOnce` false
          (:`Completed`
            (bind _returnvalue (`|AddComponentByClass` (`self.As RTSCamera`) "/Script/Engine.StaticMeshComponent" false (`self.Build Preview Transform`)))
            (set `self.PreviewMesh` _returnvalue))))
      (:`then_1`
        (set `self.Build Preview Transform` (`KismetMathLibrary.MakeTransform` (`.Location` (`GameplayStatics.BreakHitResult` _outhit))))))))