(event `self.ReceiveBeginPlay`
  (bind _asrtscamera (cast `/Game/RTSCamera/RTSCamera` (`Actor.GetOwner`)))
  (set `self.Camera` (`/Game/RTSCamera/RTSCamera.Camera` _asrtscamera)))

(event `Preview Loop`
  (bind (_returnvalue_location _returnvalue_rotation) (`KismetMathLibrary.BreakTransform` (`SceneComponent.K2_GetComponentToWorld` (`self.Camera`))))
  (bind _outhit (`KismetSystemLibrary.LineTraceSingle` :`Start` _returnvalue_location :`End` (+ _returnvalue_location (* (`KismetMathLibrary.GetForwardVector` _returnvalue_rotation) 700.0)) :`TraceChannel` "TraceTypeQuery1" :`DrawDebugType` "ForDuration"))
  (if true
    (`/Engine/EditorBlueprintResources/StandardMacros.DoOnce` false)))